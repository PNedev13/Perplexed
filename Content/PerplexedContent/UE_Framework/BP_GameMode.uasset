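; Game mode that handles the main menu and the transition into gameplay.
; On BeginPlay it creates and registers a Blueprint implementables library instance, then shows the MainMenu widget with UI-only input and a visible cursor.
; On game start it spawns BP_Character at a fixed location, possesses it with movement disabled and eases the view to it, calling StartGame after a matching delay.
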(event Custom|OnStartGame
  (Utilities|OnStartGame))

(event EventBeginPlay
  (Utilities|FlowControl|Sequence
    (:then_0
      ;[1 1 1] Create BP Library
      (bind _returnvalue (Game|ConstructObjectfromClass "/Game/PerplexedContent/BP_BPImplementablesLibrary.BP_BPImplementablesLibrary_C" self))
      (Variables|Default|SetBPImplementablesLibrary _returnvalue)
      (Class|BPImplementablesLibrary|SetInstance _returnvalue))
    (:then_1
      (Utilities|CreateMainMenu))))

(event EventTick
  (params (DeltaSeconds :type Float%20%28single-precision%29)))

(fn ConstructionScript)